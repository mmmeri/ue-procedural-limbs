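; BP_Headsneak is a player-controlled six-limbed creature whose arms are animated procedurally.
; The construction script adds a limb animator for each left and right front, center and back arm, tagged by side and level, then a coordinator linking them to the Cube root body.
; Tick applies swept movement from input, with Shift sprint and hold-to-rise jump, plus yaw turning, all gated by CanMove.
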(event `self.ReceiveTick`
  (params (DeltaSeconds :type "Float (single-precision)"))
  (if (`self.Can Move?`)
    (`|ExecutionSequence`
      (:`then_0`
        (`self.K2_AddActorWorldOffset` (* (+ (* (`KismetMathLibrary.Normal` (+ (`self.ForwardInput`) (`self.RightInput`))) (* (`self.Movement Speed`) (`self.Sprint Multiplier`))) (`self.JumpInput`)) (`GameplayStatics.GetWorldDeltaSeconds`)) true))
      (:`then_1`
        (`self.K2_AddActorWorldRotation` (`KismetMathLibrary.MakeRotator` 0.0 0.0 (* (* (`self.Rotation Input`) (`self.Rotation Speed`)) (`GameplayStatics.GetWorldDeltaSeconds`))))))))

(event `InputAction|Jump`
  (params (Key :type "Key Structure"))
  ;[1 1 1] Input Events
  (:`Pressed`
    (set `self.JumpInput` (* (`self.GetActorUpVector`) 500.0)))
  (:`Released`
    (set `self.JumpInput` (0.0 0.0 0.0))))

(event `Key|LeftShift`
  (params (Key :type "Key Structure"))
  ;[1 1 1] Input Events
  (:`Pressed`
    (set `self.Sprint Multiplier` 2.3))
  (:`Released`
    (set `self.Sprint Multiplier` 1.0)))

(event `InputAxis|MoveForward`
  (params (AxisValue :type "Float (single-precision)"))
  ;[1 1 1] Input Events
  (set `self.ForwardInput` (* (`self.GetActorForwardVector`) AxisValue)))

(event `InputAxis|MoveRight`
  (params (AxisValue :type "Float (single-precision)"))
  ;[1 1 1] Input Events
  (set `self.RightInput` (* (`self.GetActorRightVector`) AxisValue)))

(event `InputAxis|Turn`
  (params (AxisValue :type "Float (single-precision)"))
  ;[1 1 1] Input Events
  (set `self.Rotation Input` AxisValue))

(fn `Set Can Move`
  (params (`Can Move?` :type Boolean))
  (set `self.Can Move?` `Can Move?`))

(fn `UserConstructionScript`
  (`|ExecutionSequence`
    (:`then_0`
      (`AddComponent|NODE_AddAComp_LimbAnimator-1` :`SkeletalMesh` (`self.Arm RightFront`) :`Target Trace Source` (`self.RightFront`) :`Side` "NewEnumerator3")
      (`AddComponent|NODE_AddAComp_LimbAnimator-2` :`SkeletalMesh` (`self.Arm RightBack`) :`Target Trace Source` (`self.RightBack`) :`Side` "NewEnumerator3" :`Level` 2)
      (`AddComponent|NODE_AddAComp_LimbAnimator-3` :`SkeletalMesh` (`self.Arm LeftFront`) :`Target Trace Source` (`self.LeftFront`))
      (`AddComponent|NODE_AddAComp_LimbAnimator-4` :`SkeletalMesh` (`self.Arm LeftBack`) :`Target Trace Source` (`self.LeftBack`) :`Level` 2)
      (`AddComponent|NODE_AddAComp_LimbAnimator-5` :`SkeletalMesh` (`self.Arm LeftCenter`) :`Target Trace Source` (`self.LeftCenter`) :`Level` 1)
      (`AddComponent|NODE_AddAComp_LimbAnimator-6` :`SkeletalMesh` (`self.Arm RightCenter`) :`Target Trace Source` (`self.RightCenter`) :`Side` "NewEnumerator3" :`Level` 1))
    (:`then_1`
      (`AddComponent|NODE_AddAComp_LimbCoordinator-0` :`Limb Animator Components` (`self.K2_GetComponentsByClass` "/Game/ProceduralAnimation/AComp_LimbAnimator.AComp_LimbAnimator_C") :`RootBody` (`self.Cube`)))))